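; Lane-based track tile that spawns its obstacles, requests further lanes and cleans itself up as the player character passes.
; BeginPlay sets up lanes and generates obstacles from the game mode's tile count.
; Once that count exceeds three, items are attached to the platform and a timeline animates its height and pitch into place.
; Character overlap with the spawn trigger calls SpawnLanes; leaving the end trigger destroys the tile after a short delay.
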(event OnComponentEndOverlap(EndTileCollision)
  (params (OverlappedComponent :type Primitive%20Component%20Object%20Reference) (OtherActor :type Actor%20Object%20Reference) (OtherComp :type Primitive%20Component%20Object%20Reference) (OtherBodyIndex :type Integer))
  (Utilities|Casting|CastToThirdPersonCharacter OtherActor)
  (Utilities|FlowControl|Delay 1.5)
  (Actor|DestroyActor))

(event OnComponentBeginOverlap(SpawnTileCollision)
  (params (OverlappedComponent :type Primitive%20Component%20Object%20Reference) (OtherActor :type Actor%20Object%20Reference) (OtherComp :type Primitive%20Component%20Object%20Reference) (OtherBodyIndex :type Integer) (bFromSweep :type Boolean) (SweepResult :type Hit%20Result%20Structure%20%28by%20ref%29))
  (Utilities|Casting|CastToThirdPersonCharacter OtherActor)
  (bind _asthird_person_game_mode (Utilities|Casting|CastToThirdPersonGameMode (Game|GetGameMode)))
  (Default|SpawnLanes _asthird_person_game_mode))

(event EventBeginPlay
  (bind _platformscene (Variables|Default|GetPlatformScene))
  (bind _platformscene_2 (Variables|Default|GetPlatformScene))
  (bind _returnvalue (Transformation|GetWorldLocation _platformscene))
  (bind _returnvalue_2 (Transformation|GetWorldLocation _platformscene_2))
  (CallFunction|SetupLanes)
  (bind _asthird_person_game_mode (Utilities|Casting|CastToThirdPersonGameMode (Game|GetGameMode)))
  (CallFunction|GenerateObstacle (Variables|/Game/ThirdPersonBP/Blueprints/ThirdPersonGameMode.ThirdPersonGameMode_C|GetTilesCount _asthird_person_game_mode))
  (if (> (Variables|/Game/ThirdPersonBP/Blueprints/ThirdPersonGameMode.ThirdPersonGameMode_C|GetTilesCount _asthird_person_game_mode) 3)
    (Variables|Default|SetSpawnZ (.z _returnvalue_2))
    (for _array_element (Variables|Default|GetItemsList)
      (if (Utilities|IsValid _array_element)
        (Transformation|AttachComponentToComponent _array_element (Variables|Default|GetPlatformScene) "None" "KeepWorld" "SnapToTarget" "KeepWorld" true)))
    (Transformation|SetWorldLocation (Variables|Default|GetPlatformScene) (Math|Vector|MakeVector (.x _returnvalue_2) (.y _returnvalue_2) (Variables|Default|GetCurrentZ)) false false)
    (bind _newtrack_0 (Timeline|Timeline_0 PlayFromStart)
      (:Update
        (Transformation|SetWorldLocationAndRotation (Variables|Default|GetPlatformScene) (Math|Vector|MakeVector (.x _returnvalue) (.y _returnvalue) (Math|Float|Lerp (+ (Variables|Default|GetSpawnZ) 2.3e+03) (Variables|Default|GetSpawnZ) _newtrack_0)) (Math|Rotator|MakeRotator 0.0 (Math|Float|Lerp 9e+01 0.0 _newtrack_0) 0.0) false false)))))

(event EventTick
  (params (DeltaSeconds :type Float%20%28single-precision%29))
  (|CallParentFunction DeltaSeconds) ; This node is disabled and will not be called.\nDrag off pins to build functionality.
)

(fn ConstructionScript
  (|CallParentFunction))