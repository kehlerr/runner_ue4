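; GapTile is a track tile for an endless runner that advances lane spawning and speeds up the player.
; Character overlap with SpawnNewCollision calls the game mode's SpawnLanes, raises walk speed within limits, then destroys the tile after a delay.
; Leaving EndTileCollision also triggers delayed destruction, and Destroyed cleans up ItemsList actors.
; Weighted random obstacle and coin generation per shuffled lane exists, but its entry chain is disconnected.
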(event OnComponentBeginOverlap(SpawnNewCollision)
  (params (OverlappedComponent :type Primitive%20Component%20Object%20Reference) (OtherActor :type Actor%20Object%20Reference) (OtherComp :type Primitive%20Component%20Object%20Reference) (OtherBodyIndex :type Integer) (bFromSweep :type Boolean) (SweepResult :type Hit%20Result%20Structure%20%28by%20ref%29))
  (Utilities|Casting|CastToThirdPersonCharacter OtherActor)
  (bind _asthird_person_game_mode (Utilities|Casting|CastToThirdPersonGameMode (Game|GetGameMode)))
  (Default|SpawnLanes _asthird_person_game_mode)
  (bind _asthird_person_character (Utilities|Casting|CastToThirdPersonCharacter (Game|GetPlayerCharacter 0)))
  (Variables|/Script/Engine.CharacterMovementComponent|SetMaxWalkSpeed (Variables|/Script/Engine.Character|GetCharacterMovement _asthird_person_character) (Math|Float|Clamp(Float) (* (Variables|/Script/Engine.CharacterMovementComponent|GetMaxWalkSpeed (Variables|/Script/Engine.Character|GetCharacterMovement _asthird_person_character)) 1.02) 6e+02 1.5e+03))
  (Utilities|FlowControl|Delay 0.5)
  (Actor|DestroyActor))

(event OnComponentEndOverlap(EndTileCollision)
  (params (OverlappedComponent :type Primitive%20Component%20Object%20Reference) (OtherActor :type Actor%20Object%20Reference) (OtherComp :type Primitive%20Component%20Object%20Reference) (OtherBodyIndex :type Integer))
  (Utilities|FlowControl|Delay 0.5)
  (Actor|DestroyActor))

(event EventBeginPlay)

(event EventDestroyed
  ;[1 1 1] Delete items spawned on this tile
  (for _array_element (Variables|Default|GetItemsList)
    (Utilities|IsValid _array_element
      (:Is%20Valid
        (Actor|DestroyActor _array_element)))))

(event EventTick
  (params (DeltaSeconds :type Float%20%28single-precision%29)))

(event Collision|EventActorBeginOverlap
  (params (OtherActor :type Actor%20Object%20Reference)))

(fn ConstructionScript)

(fn GenerateObstacle
  (params (TilesCount :type Integer))
  (bind _lanes (Variables|Default|GetLanes))
  (if (> TilesCount (LocalVariables|Getminimum%20tiles%20to%20generate%20obstacle))
    (if (> TilesCount 100)
      (LocalVariables|Setmax%20spawn%20probability 0.75))
    (LocalVariables|Setcurrent%20spawn%20probability (Math|Random|RandomFloatinRange 0.05 (LocalVariables|Getmax%20spawn%20probability)))
    (Utilities|Array|Shuffle _lanes)
    (for (_ _array_index) _lanes
      (if (Math|Random|RandomBoolwithWeight (LocalVariables|Getcurrent%20spawn%20probability))
        (switch int (Math|Random|RandomInteger 4)
          (:Default
            (LocalVariables|SetObstacle%20Class 0 :!label _label))
          (:0
            (LocalVariables|SetObstacle%20Class "/Game/Assets/Blueprints/Obstacle_pipe.Obstacle_pipe_C"))
          (:1
            (LocalVariables|SetObstacle%20Class "/Game/Assets/Blueprints/Obstacle_Box.Obstacle_Box_C"))
          (:2
            (LocalVariables|SetObstacle%20Class "/Game/Assets/Blueprints/Obstacle_high_pipe.Obstacle_high_pipe_C"))
          (:3
            (LocalVariables|SetObstacle%20Class "/Game/Assets/Blueprints/Reward_coin.Reward_coin_C")))
        (else
          (LocalVariables|Setcurrent%20spawn%20probability (* (LocalVariables|Getcurrent%20spawn%20probability) 2.0))
          (goto _label)))
      (Utilities|Array|Insert (Variables|Default|GetObstaclesByLanes) (LocalVariables|GetObstacle%20Class) _array_index))
    (CallFunction|SpawnItems)))

(fn GenerateReward
  (params (LaneTransform :type Transform))
  (bind _returnvalue (Game|SpawnActorfromClass (LocalVariables|Getreward%20coin%20class) LaneTransform "Undefined" 0 0))
  (Utilities|Array|Add (Variables|Default|GetItemsList) _returnvalue))

(fn SpawnItems
  (for (_array_element _array_index) (Variables|Default|GetLanes)
    (bind _returnvalue (Game|SpawnActorfromClass (Utilities|Array|Get(acopy) (Variables|Default|GetObstaclesByLanes) _array_index) (Math|Conversions|ToTransform(Vector) (Transformation|GetWorldLocation _array_element)) "Undefined" 0 0))
    (Utilities|Array|Add (Variables|Default|GetItemsList) _returnvalue)))