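; Base track tile for an endless runner that fills its lanes with random items and cleans them up on destruction.
; BeginPlay shuffles tagged lanes and rolls boxes, coins or water drops, doubling the odds after each empty lane.
; Past 25 tiles, a timeline animates the platform and attached items into place, then requests the next tile.
; The tile self-destructs shortly after the player exits, and its deathbox triggers game loss.
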(event OnComponentEndOverlap(EndTileCollision)
  (params (OverlappedComponent :type Primitive%20Component%20Object%20Reference) (OtherActor :type Actor%20Object%20Reference) (OtherComp :type Primitive%20Component%20Object%20Reference) (OtherBodyIndex :type Integer))
  (Utilities|Casting|CastToThirdPersonCharacter OtherActor)
  (Utilities|FlowControl|Delay 1.5)
  (Actor|DestroyActor))

(event OnComponentBeginOverlap(FallDeathbox)
  (params (OverlappedComponent :type Primitive%20Component%20Object%20Reference) (OtherActor :type Actor%20Object%20Reference) (OtherComp :type Primitive%20Component%20Object%20Reference) (OtherBodyIndex :type Integer) (bFromSweep :type Boolean) (SweepResult :type Hit%20Result%20Structure%20%28by%20ref%29))
  (bind _asthird_person_game_mode (Utilities|Casting|CastToThirdPersonGameMode (Game|GetGameMode)))
  (Default|LoseGame _asthird_person_game_mode))

(event EventBeginPlay
  (bind _defaultsceneroot (Variables|Default|GetDefaultSceneRoot))
  (bind _platformscene (Variables|Default|GetPlatformScene))
  (bind _returnvalue (Transformation|GetWorldLocation _defaultsceneroot))
  (bind _returnvalue_2 (Transformation|GetWorldLocation _platformscene))
  (Variables|Default|SetLanes (Actor|GetComponentsbyTag "/Script/Engine.SceneComponent" "Lane"))
  (bind _asthird_person_game_mode (Utilities|Casting|CastToThirdPersonGameMode (Game|GetGameMode)))
  (CallFunction|GenerateObstacle (Variables|/Game/ThirdPersonBP/Blueprints/ThirdPersonGameMode.ThirdPersonGameMode_C|GetTilesCount _asthird_person_game_mode))
  (if (> (Variables|/Game/ThirdPersonBP/Blueprints/ThirdPersonGameMode.ThirdPersonGameMode_C|GetTilesCount _asthird_person_game_mode) 25)
    (Variables|Default|SetSpawnZ (.z _returnvalue_2))
    (Utilities|FlowControl|Delay 1.5)
    (for _array_element (Variables|Default|GetItemsList)
      (Transformation|AttachComponentToComponent _array_element (Variables|Default|GetPlatformScene) "None" "KeepWorld" "KeepWorld" "KeepWorld" true))
    (Transformation|SetWorldLocation (Variables|Default|GetPlatformScene) (Math|Vector|MakeVector (.x _returnvalue_2) (.y _returnvalue_2) (Variables|Default|GetCurrentZ)) false false)
    (bind _newtrack_0 (Timeline|FallingPlatformTimeline PlayFromStart)
      (:Update
        (Transformation|SetWorldLocation (Variables|Default|GetPlatformScene) (Math|Vector|MakeVector (.x _returnvalue) (.y _returnvalue) (Math|Float|Lerp (Variables|Default|GetCurrentZ) (Variables|Default|GetSpawnZ) _newtrack_0)) false false))
      (:Finished
        (bind _asthird_person_game_mode_2 (Utilities|Casting|CastToThirdPersonGameMode (Game|GetGameMode)))
        (Default|SpawnTile _asthird_person_game_mode_2 "/Game/Assets/Blueprints/Tiles/SpawnerPlaneTile.SpawnerPlaneTile_C")))))

(event EventDestroyed
  ;[1 1 1] Delete items spawned on this tile
  (for _array_element (Variables|Default|GetItemsList)
    (Utilities|IsValid _array_element
      (:Is%20Valid
        (Actor|DestroyActor _array_element)))))

(event EventTick
  (params (DeltaSeconds :type Float%20%28single-precision%29)))

(event Collision|EventActorBeginOverlap
  (params (OtherActor :type Actor%20Object%20Reference)))

(fn ConstructionScript)

(fn GenerateObstacle
  (params (TilesCount :type Integer))
  (bind _lanes (Variables|Default|GetLanes))
  (if (> TilesCount (LocalVariables|Getminimum%20tiles%20to%20generate%20obstacle))
    (if (> TilesCount 100)
      (LocalVariables|Setmax%20spawn%20probability 0.75))
    (LocalVariables|Setcurrent%20spawn%20probability (Math|Random|RandomFloatinRange 0.05 (LocalVariables|Getmax%20spawn%20probability)))
    (Utilities|Array|Shuffle _lanes)
    (for (_ _array_index) _lanes
      (if (Math|Random|RandomBoolwithWeight (LocalVariables|Getcurrent%20spawn%20probability))
        (switch int (Math|Random|RandomInteger 3)
          (:Default
            (LocalVariables|SetObstacle%20Class "/Game/Assets/Blueprints/Obstacles/Obstacle_Box.Obstacle_Box_C"))
          (:0
            (LocalVariables|SetObstacle%20Class "/Game/Assets/Blueprints/Items/Reward_coin.Reward_coin_C"))
          (:1
            (LocalVariables|SetObstacle%20Class "/Game/Assets/Blueprints/Items/WaterDrop.WaterDrop_C")))
        (else
          (LocalVariables|Setcurrent%20spawn%20probability (* (LocalVariables|Getcurrent%20spawn%20probability) 2.0))
          (LocalVariables|SetObstacle%20Class 0)))
      (Utilities|Array|Insert (Variables|Default|GetObstaclesByLanes) (LocalVariables|GetObstacle%20Class) _array_index))
    (CallFunction|SpawnItems)))

(fn GenerateReward
  (params (LaneTransform :type Transform))
  (bind _returnvalue (Game|SpawnActorfromClass (LocalVariables|Getreward%20coin%20class) LaneTransform "Undefined" 0 0))
  (Utilities|Array|Add (Variables|Default|GetItemsList) _returnvalue))

(fn SpawnItems
  (for (_array_element _array_index) (Variables|Default|GetLanes)
    (bind _returnvalue (Game|SpawnActorfromClass (Utilities|Array|Get(acopy) (Variables|Default|GetObstaclesByLanes) _array_index) (Math|Conversions|ToTransform(Vector) (Transformation|GetWorldLocation _array_element)) "Undefined" 0 0))
    (Utilities|Array|Add (Variables|Default|GetItemsList) _returnvalue)))

(fn SetupLanes
  (bind _asthird_person_game_mode (Utilities|Casting|CastToThirdPersonGameMode (Game|GetGameMode)))
  (if (> (Variables|/Game/ThirdPersonBP/Blueprints/ThirdPersonGameMode.ThirdPersonGameMode_C|GetTilesCount _asthird_person_game_mode) 10)
    (switch int (Math|Random|RandomInteger 10)
      (:Default
        _)
      (:0
        (Components|DestroyComponent (Variables|Default|GetCube)))
      (:1
        (Components|DestroyComponent (Variables|Default|GetCube1)))
      (:2
        (Components|DestroyComponent (Variables|Default|GetCube2)))))
  (Variables|Default|SetLanes (Actor|GetComponentsbyTag "/Script/Engine.SceneComponent" "ItemSpawn")))