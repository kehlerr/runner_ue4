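; Obstacle box that changes the score when a ThirdPersonCharacter overlaps its CollisionBox.
; It adds PointsChange to Points on the ThirdPersonGameMode, clamped between zero and the current total, so the box can only lower the score.
; It then hides Cube and shows CubeEaten, leaving collision untouched, so later overlaps apply the change again.
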(event OnComponentBeginOverlap(CollisionBox)
  (params (OverlappedComponent :type Primitive%20Component%20Object%20Reference) (OtherActor :type Actor%20Object%20Reference) (OtherComp :type Primitive%20Component%20Object%20Reference) (OtherBodyIndex :type Integer) (bFromSweep :type Boolean) (SweepResult :type Hit%20Result%20Structure%20%28by%20ref%29))
  (Utilities|Casting|CastToThirdPersonCharacter OtherActor)
  (bind _asthird_person_game_mode (Utilities|Casting|CastToThirdPersonGameMode (Game|GetGameMode)))
  (Variables|/Game/ThirdPersonBP/Blueprints/ThirdPersonGameMode.ThirdPersonGameMode_C|SetPoints _asthird_person_game_mode (Math|Integer|Clamp(Integer) (+ (Variables|Default|GetPointsChange) (Variables|/Game/ThirdPersonBP/Blueprints/ThirdPersonGameMode.ThirdPersonGameMode_C|GetPoints _asthird_person_game_mode)) 0 (Variables|/Game/ThirdPersonBP/Blueprints/ThirdPersonGameMode.ThirdPersonGameMode_C|GetPoints _asthird_person_game_mode)))
  (Rendering|SetVisibility (Variables|Default|GetCube) false false)
  (Rendering|SetVisibility (Variables|Default|GetCubeEaten) true false))

(event EventBeginPlay)

(event Collision|EventActorBeginOverlap
  (params (OtherActor :type Actor%20Object%20Reference)))

(event EventTick
  (params (DeltaSeconds :type Float%20%28single-precision%29)))

(fn ConstructionScript)