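; High pipe obstacle actor that kills the third-person character when the two overlap.
; On overlap it calls the character's DeathFunction, plays a crash splash sound and drops global time dilation into slow motion.
; After a short delay, stretched by that dilation, it destroys the character; time dilation is not restored here.
; An unconnected older branch would instead deduct a game mode point and destroy the obstacle.
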(event EventBeginPlay)

(event Collision|EventActorBeginOverlap
  (params (OtherActor :type Actor%20Object%20Reference))
  (bind _asthird_person_character (Utilities|Casting|CastToThirdPersonCharacter OtherActor))
  (Default|DeathFunction _asthird_person_character)
  (Audio|SpawnSound2D "/Game/Assets/SFX/crash_splash.crash_splash" 1.0 1.0 0.0 0)
  (Utilities|Time|SetGlobalTimeDilation 0.1)
  (Utilities|FlowControl|Delay 0.2)
  (Actor|DestroyActor _asthird_person_character))

(event EventTick
  (params (DeltaSeconds :type Float%20%28single-precision%29)))

(fn ConstructionScript)