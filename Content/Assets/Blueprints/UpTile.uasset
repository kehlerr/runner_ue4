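; UpTile is a tile Blueprint that sets up per-lane obstacles for a lane-based level.
; On BeginPlay it gathers scene components tagged "Lane" and adds an Obstacle_Box entry to ObstaclesByLanes for each one.
; It then calls SpawnItems, whose logic is not defined in this file.
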(event EventBeginPlay
  (bind _output_get (Variables|Default|SetLanes (Actor|GetComponentsbyTag "/Script/Engine.SceneComponent" "Lane")))
  (for _array_element _output_get
    (Utilities|Array|Add (Variables|Default|GetObstaclesByLanes) "/Game/Assets/Blueprints/Obstacle_Box.Obstacle_Box_C"))
  (CallFunction|SpawnItems))

(event Collision|EventActorBeginOverlap
  (params (OtherActor :type Actor%20Object%20Reference))
  (|CallParentFunction OtherActor) ; This node is disabled and will not be called.\nDrag off pins to build functionality.
)

(event EventTick
  (params (DeltaSeconds :type Float%20%28single-precision%29))
  (|CallParentFunction DeltaSeconds) ; This node is disabled and will not be called.\nDrag off pins to build functionality.
)

(fn ConstructionScript
  (|CallParentFunction))