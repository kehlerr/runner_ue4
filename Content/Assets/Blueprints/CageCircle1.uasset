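; CageCircle1 is an actor that keeps pace with the player's hamster along the X axis while spinning.
; Each tick it casts the player character to ThirdPersonCharacter and moves its root to a fixed X offset from the hamster mesh, with constant Y and Z.
; It also sets its RotatingMovement rate on one axis in proportion to the character's MaxWalkSpeed, so spin follows the speed setting rather than actual velocity.
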(event EventBeginPlay)

(event Collision|EventActorBeginOverlap
  (params (OtherActor :type Actor%20Object%20Reference)))

(event EventTick
  (params (DeltaSeconds :type Float%20%28single-precision%29))
  (bind _asthird_person_character (Utilities|Casting|CastToThirdPersonCharacter (Game|GetPlayerCharacter 0)))
  (Transformation|SetWorldLocation (Variables|Default|GetDefaultSceneRoot) (Math|Vector|MakeVector (+ (.x (.location (Transformation|GetWorldTransform (Variables|/Game/ThirdPersonBP/Blueprints/ThirdPersonCharacter.ThirdPersonCharacter_C|GetStaticMeshHamster _asthird_person_character)))) 2e+02) -6e+02 2.5e+03) false false)
  (Variables|/Script/Engine.RotatingMovementComponent|SetRotationRate (Variables|Default|GetRotatingMovement) (Math|Rotator|MakeRotator 0.0 (/ (Variables|/Script/Engine.CharacterMovementComponent|GetMaxWalkSpeed (Variables|/Script/Engine.Character|GetCharacterMovement _asthird_person_character)) 5e+02) 0.0)))

(fn ConstructionScript)